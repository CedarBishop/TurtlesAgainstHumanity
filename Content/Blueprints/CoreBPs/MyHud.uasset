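; MyHud is the game's HUD Blueprint, creating and managing the on-screen widgets for each level.
; On BeginPlay it switches on level name: gameplay levels get oxygen bar, breaking news, screen blur and hidden pause menu, the main menu gets its menu, and the transition level a serious message.
; Gameplay levels and the main menu also share a hidden settings widget.
; Custom events forward breaking news and toggle visibility between pause, main and settings menus.
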(event Custom|SpawnBreakingNews
  (params (BreakingNews :type String))
  (Default|CycleNewsList (Variables|Default|GetBreakingNewsWidget) BreakingNews))

(event Custom|SetPauseState
  (params (IsPaused :type Boolean))
  (bind _pausemenuwidget (Variables|Default|GetPauseMenuWidget))
  (if IsPaused
    (Widget|SetVisibility _pausemenuwidget "Visible")
    (else
      (Widget|SetVisibility _pausemenuwidget "Hidden"))))

(event Custom|PauseSettingsSwitch
  (params (SwitchToSettings :type Boolean))
  (bind _pausemenuwidget (Variables|Default|GetPauseMenuWidget))
  (bind _settingsmenuwidget (Variables|Default|GetSettingsMenuWidget))
  (if SwitchToSettings
    (Widget|SetVisibility _pausemenuwidget "Hidden")
    (Widget|SetVisibility _settingsmenuwidget "Visible")
    (else
      (Widget|SetVisibility _pausemenuwidget "Visible")
      (Widget|SetVisibility _settingsmenuwidget "Hidden"))))

(event Custom|MainMenuSettingsSwitch
  (params (SwitchToSettings :type Boolean))
  (bind _settingsmenuwidget (Variables|Default|GetSettingsMenuWidget))
  (bind _mainmenuwidget (Variables|Default|GetMainMenuWidget))
  (if SwitchToSettings
    (Widget|SetVisibility _mainmenuwidget "Hidden")
    (Widget|SetVisibility _settingsmenuwidget "Visible")
    (else
      (Widget|SetVisibility _mainmenuwidget "Visible")
      (Widget|SetVisibility _settingsmenuwidget "Hidden"))))

(event EventBeginPlay
  (bind _returnvalue (Game|GetCurrentLevelName true))
  (switch string _returnvalue
    (:LevelOne
      (bind _returnvalue_2 (UserInterface|CreateWidget "/Game/Blueprints/Widgets/Widget_OxygenBar.Widget_OxygenBar_C" :!label _label))
      (UserInterface|Viewport|AddtoViewport _returnvalue_2 0)
      (bind _returnvalue_3 (UserInterface|CreateWidget "/Game/Blueprints/Widgets/Widget_BreakingNews.Widget_BreakingNews_C"))
      (bind _output_get (Variables|Default|SetBreakingNewsWidget _returnvalue_3))
      (UserInterface|Viewport|AddtoViewport _output_get 0)
      (bind _returnvalue_4 (UserInterface|CreateWidget "/Game/Blueprints/Widgets/Widget_ScreenBlur.Widget_ScreenBlur_C"))
      (bind _output_get_2 (Variables|Default|SetScreenBlurWidget _returnvalue_4))
      (UserInterface|Viewport|AddtoViewport _output_get_2 0)
      (bind _returnvalue_5 (UserInterface|CreateWidget "/Game/Blueprints/Widgets/Widget_PauseMenu.Widget_PauseMenu_C"))
      (bind _output_get_3 (Variables|Default|SetPauseMenuWidget _returnvalue_5))
      (UserInterface|Viewport|AddtoViewport _output_get_3 0)
      (Widget|SetVisibility _returnvalue_5 "Hidden")
      (bind _returnvalue_6 (UserInterface|CreateWidget "/Game/Blueprints/Widgets/Widget_Settings.Widget_Settings_C" :!label _label_2))
      (bind _output_get_4 (Variables|Default|SetSettingsMenuWidget _returnvalue_6))
      (UserInterface|Viewport|AddtoViewport _output_get_4 0)
      (Widget|SetVisibility _output_get_4 "Hidden"))
    (:LevelTwo
      (goto _label))
    (:MainMenu
      (bind _returnvalue_7 (UserInterface|CreateWidget "/Game/Blueprints/Widgets/Widget_MainMenu.Widget_MainMenu_C"))
      (UserInterface|Viewport|AddtoViewport _returnvalue_7 0)
      (Variables|Default|SetMainMenuWidget _returnvalue_7)
      (goto _label_2))
    (:TransistionLevel
      (bind _returnvalue_8 (UserInterface|CreateWidget "/Game/Blueprints/Widgets/Widget_SeriousMessage.Widget_SeriousMessage_C"))
      (UserInterface|Viewport|AddtoViewport _returnvalue_8 0))))

(fn ConstructionScript)