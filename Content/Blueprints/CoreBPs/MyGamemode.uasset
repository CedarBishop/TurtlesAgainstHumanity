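; Game mode for a PC/VR turtle game, managing menu, pollution events and endings across two playthrough levels.
; Level One starts in the menu, and death there loads a transition level; Level Two raises stress and opens the ending after a timer.
; CallEvent shows breaking news, then uses the event number to add and later remove hazards, shifting minimum stress and signalling climate change.
; Obstacles spawn randomly ahead of the turtle, plastic bags as AI around it.
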(event Custom|StartedActualGame
  (bind _returnvalue (Game|GetPlayerController 0))
  (bind _asmy_hud (Utilities|Casting|CastToMyHud (HUD|GetHUD _returnvalue)))
  (Default|StartActualGame _asmy_hud)
  (bind _asplayer_base (Utilities|Casting|CastToPlayer_Base (Game|Player|GetPlayerPawn 0)))
  (Class|PlayerBase|SetTutorialStatus _asplayer_base true)
  (Variables|/Script/VrTest.Player_Base|SetbIsInMainMenu _asplayer_base false)
  (Variables|/Script/Engine.PlayerController|SetbShowMouseCursor _returnvalue false)
  (Input|SetInputModeGameOnly _returnvalue)
  (Variables|Default|SetbIsInMainMenu false))

(event Custom|SendUnPauseMessage
  (switch Utilities|FlowControl|Switch|SwitchonCurrentPlayerController (Variables|Default|GetCurrentPlayer)
    (:NewEnumerator0
      (Default|UnPause (Variables|Default|GetPCPlayer)))
    (:NewEnumerator1
      (Default|UnPause (Variables|Default|GetVRPlayer)))))

(event Custom|PlayerDied
  (if (Variables|Default|GetbIsFirstPlaythough)
    (Variables|/Script/VrTest.LastSwim_GameInstance|SetbFirstPlaythrough (Variables|Default|GetgameInstance) false)
    (Game|OpenLevel(byName) "TransistionLevel")
    (else
      (Development|PrintString "Died in good playthrough, teleport to goal"))))

(event EventBeginPlay
  (bind _returnvalue (Game|Player|GetPlayerPawn 0))
  (bind _returnvalue_2 (Game|GetPlayerController 0))
  ;[1 1 1] Initializes the first playthrough boolean, then sets the current player controller enum based on the string value in the default pawn of gamemode. the previous position variable is then initialized to starting location
  (Utilities|FlowControl|Sequence
    (:then_0
      (bind _returnvalue_3 (Game|GetCurrentLevelName true))
      (switch string _returnvalue_3
        (:LevelOne
          (Variables|Default|SetbIsFirstPlaythough true))
        (:LevelTwo
          (Variables|Default|SetbIsFirstPlaythough false)))
      (switch Utilities|FlowControl|Switch|SwitchonCurrentPlayerController "NewEnumerator0"
        (:NewEnumerator0
          (Variables|Default|SetCurrentPlayer "NewEnumerator0")
          (bind _asbp_turtle_pc (Utilities|Casting|CastToBP_Turtle_PC _returnvalue))
          (bind _output_get (Variables|Default|SetPCPlayer _asbp_turtle_pc))
          (Variables|Default|SetplayerLastPosition (Transformation|GetActorLocation _output_get)))
        (:NewEnumerator1
          (Variables|Default|SetCurrentPlayer "NewEnumerator1")
          (bind _asbp_turtle_vr (Utilities|Casting|CastToBP_Turtle_VR _returnvalue))
          (bind _output_get_2 (Variables|Default|SetVRPlayer _asbp_turtle_vr))
          (Variables|Default|SetplayerLastPosition (Transformation|GetActorLocation _output_get_2)))))
    (:then_1
      (bind _returnvalue_4 (Game|GetCurrentLevelName true))
      (switch string _returnvalue_4
        (:LevelOne
          (Input|SetInputModeUIOnly _returnvalue_2 0 "DoNotLock")
          (Variables|/Script/Engine.PlayerController|SetbShowMouseCursor _returnvalue_2 true)
          (Variables|Default|SetbIsInMainMenu true)
          (bind _asplayer_base (Utilities|Casting|CastToPlayer_Base (Game|Player|GetPlayerPawn 0)))
          (Variables|/Script/VrTest.Player_Base|SetbIsInMainMenu _asplayer_base true))
        (:LevelTwo
          (Input|SetInputModeGameOnly _returnvalue_2)
          (Variables|/Script/Engine.PlayerController|SetbShowMouseCursor _returnvalue_2 false)
          (CallFunction|RaisePlayerMinStress 4e+01)
          (Utilities|FlowControl|Delay (Variables|Default|GetEndTimer))
          (CallFunction|PlayEndSequence))))))

(event EventExecuteCallEvent
  (CallFunction|CallEvent))

(fn ConstructionScript)

(fn CallEvent
  (bind _currentbreakingnewstext (Variables|Default|GetcurrentBreakingNewsText))
  (bind _asmy_hud (Utilities|Casting|CastToMyHud (HUD|GetHUD (Game|GetPlayerController 0))))
  (if (Utilities|Enum|NotEqual(Enum) _currentbreakingnewstext "")
    (Default|SpawnBreakingNews _asmy_hud _currentbreakingnewstext))
  (switch int (Variables|Default|GetcurrentEventNumber)
    (:Default
      (CallFunction|SpawnObstacles)
      (CallFunction|RaisePlayerMinStress 1.0))
    (:1
      (CallFunction|RaisePlayerMinStress 5.0)
      (CallFunction|SpawnPlasticBags)
      (Default|CallClimateChange))
    (:2
      (CallFunction|AddNewObstacleType "/Game/Blueprints/EnvironmentBPs/BP_HunterNets.BP_HunterNets_C")
      (CallFunction|SpawnObstacles)
      (CallFunction|RaisePlayerMinStress 5.0)
      (Default|CallClimateChange))
    (:3
      (CallFunction|AddNewObstacleType "/Game/Blueprints/EnvironmentBPs/BP_ChemicalWaste.BP_ChemicalWaste_C")
      (CallFunction|SpawnObstacles)
      (CallFunction|RaisePlayerMinStress 5.0)
      (Default|CallClimateChange))
    (:4
      (CallFunction|AddNewObstacleType "/Game/Blueprints/EnvironmentBPs/BP_OilBarrel.BP_OilBarrel_C")
      (CallFunction|SpawnObstacles)
      (CallFunction|RaisePlayerMinStress 5.0)
      (Default|CallClimateChange))
    (:5
      (CallFunction|RaisePlayerMinStress -1e+01)
      (CallFunction|RemoveObstacles "/Game/Blueprints/EnvironmentBPs/BP_OilBarrel.BP_OilBarrel_C")
      (Default|CallClimateChange))
    (:6
      (CallFunction|RaisePlayerMinStress -1e+01)
      (CallFunction|RemoveObstacles "/Game/Blueprints/EnvironmentBPs/BP_ChemicalWaste.BP_ChemicalWaste_C")
      (Default|CallClimateChange))
    (:7
      (CallFunction|RaisePlayerMinStress -1e+01)
      (CallFunction|RemoveObstacles "/Game/Blueprints/EnvironmentBPs/BP_HunterNets.BP_HunterNets_C")
      (Default|CallClimateChange))
    (:8
      (CallFunction|RaisePlayerMinStress -1e+01)
      (CallFunction|RemovePlasticBags)
      (Default|CallClimateChange))
    (:9
      (CallFunction|PlayEndSequence))))

(fn SpawnObstacles
  (bind _listofobstacles (Variables|Default|GetListOfObstacles))
  (bind _pcplayer (Variables|Default|GetPCPlayer))
  (switch Utilities|FlowControl|Switch|SwitchonCurrentPlayerController (Variables|Default|GetCurrentPlayer)
    (:NewEnumerator0
      (LocalVariables|SetObstacle%20Origin (+ (* (Math|Vector|GetForwardVector (Transformation|GetActorRotation _pcplayer)) (Variables|Default|GetObstacleForwardOffset)) (Transformation|GetActorLocation _pcplayer))))
    (:NewEnumerator1
      (LocalVariables|SetObstacle%20Origin (+ (Transformation|GetActorLocation) (* (Math|Vector|GetForwardVector (Transformation|GetActorRotation (Variables|Default|GetVRPlayer))) (Variables|Default|GetObstacleForwardOffset))))))
  (for _index (range 0 (Math|Random|RandomIntegerinRange (Variables|Default|GetminSpawnObstacles) (Variables|Default|GetmaxSpawnObstacles)))
    (bind _returnvalue (Class|LastSwimGameModeBase|GetRandomLocationinRadius (Variables|Default|GetmaxSpawnDistanceRadius) (LocalVariables|GetObstacle%20Origin) 1e+03))
    (Game|SpawnActorfromClass (Utilities|Array|Get(acopy) _listofobstacles (Math|Random|RandomInteger (Utilities|Array|Length _listofobstacles))) (Math|Transform|MakeTransform _returnvalue "0, 0, 0" "3.000000,3.000000,3.000000") "Undefined" 0 0)))

(fn ReturnRandomLocationinRadius
  (params (Radius :type Float%20%28single-precision%29) (Origin :type Vector) (Height :type Float%20%28single-precision%29))
  (bind (_x _y) (Math|Vector|BreakVector Origin))
  (return (Math|Vector|MakeVector (Math|Random|RandomFloatinRange (- _x Radius) (+ _x Radius)) (Math|Random|RandomFloatinRange (- _y Radius) (+ _y Radius)) Height)))

(fn SpawnGoal
  (bind _returnvalue (Class|LastSwimGameModeBase|GetRandomLocationinRadius 0.0 (* (Math|Vector|GetForwardVector (Variables|/Script/VrTest.Player_Base|Getcamera (Variables|Default|Getplayer))) (LocalVariables|GetGoalSpawnDistanceFromPlayer)) 5e+02))
  (Default|CallOnSpawnGoal _returnvalue)
  (Game|SpawnActorfromClass "/Game/Blueprints/EnvironmentBPs/BP_Goal.BP_Goal_C" (Math|Transform|MakeTransform _returnvalue) "Undefined" 0 0))

(fn RaisePlayerMinStress
  (params (AddedStress :type Float%20%28single-precision%29))
  (switch Utilities|FlowControl|Switch|SwitchonCurrentPlayerController (Variables|Default|GetCurrentPlayer)
    (:NewEnumerator0
      (Default|RaiseMinStress (Variables|Default|GetPCPlayer) AddedStress))
    (:NewEnumerator1
      (Default|RaiseMinStress (Variables|Default|GetVRPlayer) AddedStress))))

(fn AddNewObstacleType
  (params (NewObstacleType :type BP%20Obstacle%20Class%20Reference))
  (Utilities|Array|Add (Variables|Default|GetListOfObstacles) NewObstacleType))

(fn ChangeMaterialQuality
  (params (newLevel :type Integer))
  (switch int newLevel
    (:0
      (Development|ExecuteConsoleCommand "r.MaterialQualityLevel 0" 0))
    (:1
      (Development|ExecuteConsoleCommand "r.MaterialQualityLevel 1" 0))
    (:2
      (Development|ExecuteConsoleCommand "r.MaterialQualityLevel 2" 0))))

(fn SpawnPlasticBags
  (for _index (range 0 20)
    (bind _returnvalue (Class|LastSwimGameModeBase|GetRandomLocationinRadius 1e+04 (Transformation|GetActorLocation (Variables|Default|Getplayer)) 5e+02))
    (AI|SpawnAIFromClass "/Game/Blueprints/EnvironmentBPs/BP_PlasticBag.BP_PlasticBag_C" "/Game/Blueprints/AIBPs/FishAI/BT_FishAI.BT_FishAI" _returnvalue "0, 0, 0" false)))

(fn RemovePlasticBags
  (bind _outactors (Actor|GetAllActorsOfClass "/Game/Blueprints/EnvironmentBPs/BP_PlasticBag.BP_PlasticBag_C"))
  (for _array_element _outactors
    (Actor|DestroyActor _array_element)))

(fn RemoveObstacles
  (params (ObstacleType :type BP%20Obstacle%20Class%20Reference))
  (bind _outactors (Actor|GetAllActorsOfClass ObstacleType))
  (for _array_element _outactors
    (Actor|DestroyActor _array_element)))

(fn PlayEndSequence
  (if (not (Variables|Default|GetPlayedEnding))
    (Variables|Default|SetPlayedEnding true)
    (Game|OpenLevel(byName) "EndingBeach")))