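; BP_FeederFishAI is the feeder fish AI character, varied per instance at spawn.
; BeginPlay gives the mesh a random uniform scale and randomizes the CharacterMovement max walk speed.
; GetClosestCoral returns the closest object from the DistanceToObjectsDetector component; its validity check has no effect, as both branches return the same result.
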(event EventBeginPlay
  (Transformation|SetRelativeScale3D (Variables|Character|GetMesh) (* (Class|KismetMathLibrary|VectorOne) (Math|Random|RandomFloatinRange 0.5 1.5)))
  (Variables|/Script/Engine.CharacterMovementComponent|SetMaxWalkSpeed (Variables|Character|GetCharacterMovement) (Math|Random|RandomFloatinRange 1.5e+02 3e+02)))

(event Collision|EventActorBeginOverlap
  (params (OtherActor :type Actor%20Object%20Reference)))

(event EventTick
  (params (DeltaSeconds :type Float%20%28single-precision%29)))

(fn ConstructionScript)

(fn GetClosestCoral
  (bind _returnvalue (Class|DistancetoObjectsDetector|GetClosestObject (Variables|Default|GetDistanceToObjectsDetector)))
  (Utilities|IsValid _returnvalue
    (:Is%20Valid
      (return _returnvalue))
    (:Is%20Not%20Valid
      (return _returnvalue))))