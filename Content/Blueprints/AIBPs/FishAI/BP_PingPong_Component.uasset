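; Scene component in the fish AI folder that drifts back and forth along a fixed diagonal in its relative X/Y plane.
; BeginPlay picks a random reversal interval and a random uniform scale, so instances vary in timing and size.
; Tick applies a constant per-frame offset without delta-time scaling, while a Delay on the same Tick flips the direction each time the interval elapses.
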(event EventBeginPlay
  (Variables|Default|SetTime (Math|Random|RandomFloatinRange 0.0 5.0))
  (Transformation|SetRelativeTransform (Math|Transform|MakeTransform (Variables|Default|GetRelativeLocation) (Variables|Default|GetRelativeRotation) (* "1.000000,1.000000,1.000000" (Math|Random|RandomFloatinRange 0.5 2.0))) false false))

(event EventTick
  (params (DeltaSeconds :type Float%20%28single-precision%29))
  (Utilities|FlowControl|Sequence
    (:then_0
      (if (Variables|Default|GetbIsGoingRight)
        (Transformation|AddRelativeLocation "-0.200000,0.400000, 0" false false)
        (else
          (Transformation|AddRelativeLocation "0.200000,-0.400000, 0" false false))))
    (:then_1
      (Utilities|FlowControl|Delay (Variables|Default|GetTime))
      (Variables|Default|SetbIsGoingRight (not (Variables|Default|GetbIsGoingRight))))))