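; BP_FishAI is a simple fish actor whose mesh continuously bobs up and down.
; Tick nudges the mesh along its relative Z axis by a fixed step each frame, so speed depends on frame rate.
; A Delay on the same Tick flips the direction after an interval randomized once at BeginPlay, so each fish reverses on its own period.
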(event EventTick
  (params (DeltaSeconds :type Float%20%28single-precision%29))
  (Utilities|FlowControl|Sequence
    (:then_0
      (if (Variables|Default|GetbIsGoingUp)
        (Transformation|AddRelativeLocation (Variables|Character|GetMesh) "0,0.000000,0.200000" false false)
        (else
          (Transformation|AddRelativeLocation (Variables|Character|GetMesh) "0,0.000000,-0.200000" false false))))
    (:then_1
      (Utilities|FlowControl|Delay (Variables|Default|GetTime))
      (Variables|Default|SetbIsGoingUp (not (Variables|Default|GetbIsGoingUp))))))

(event EventBeginPlay
  (Variables|Default|SetTime (Math|Random|RandomFloatinRange 5.0 15.0)))

(fn ConstructionScript)