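; BP_Oxygen is an oxygen pickup actor that replenishes the player's oxygen on contact.
; Overlapping a BP_IPlayer calls OnOxygenReSupply with OxygenAmount and no stress healing, then starts a timed countdown to destroy the actor.
; While the overlap lasts, Tick feeds a Delay of TimeBtwOxygen to repeat the resupply periodically.
; BeginPlay caches MyGamemode, which the graph never uses afterwards.
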(event EventBeginPlay
  (bind _asmy_gamemode (Utilities|Casting|CastToMyGamemode (Game|GetGameMode)))
  (Variables|Default|SetGamemode _asmy_gamemode))

(event Collision|EventActorBeginOverlap
  (params (OtherActor :type Actor%20Object%20Reference))
  (bind _asbp_iplayer (Utilities|Casting|CastToBP_IPlayer OtherActor))
  (bind _output_get (Variables|Default|SetPlayer _asbp_iplayer))
  (Default|OnOxygenReSupply _output_get 0.0 (Variables|Default|GetOxygenAmount))
  (Variables|Default|SetIsOverlappingPlayer true)
  (Utilities|FlowControl|Delay (Variables|Default|GetTimeToLiveAfterContact))
  (Actor|DestroyActor))

(event EventTick
  (params (DeltaSeconds :type Float%20%28single-precision%29))
  (if (Variables|Default|GetIsOverlappingPlayer)
    (Utilities|FlowControl|Delay (Variables|Default|GetTimeBtwOxygen))
    (Default|OnOxygenReSupply (Variables|Default|GetPlayer) 0.0 (Variables|Default|GetOxygenAmount))))

(event Collision|EventActorEndOverlap
  (params (OtherActor :type Actor%20Object%20Reference))
  (Utilities|Casting|CastToBP_IPlayer OtherActor)
  (Variables|Default|SetIsOverlappingPlayer false))

(fn ConstructionScript)