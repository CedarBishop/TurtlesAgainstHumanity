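; BP_EnvironmentChange shifts the scene's color mood when the game mode's ClimateChange event fires.
; On BeginPlay it caches the player pawn's camera and the first ExponentialHeightFog, then applies initial post-process and fog colors.
; Each change starts timelines that lerp camera scene tint and fog directional inscattering between adjacent color-array entries, both using the post-process timeline's alpha.
; A StartLerping flag gates changes; temperature blending and other fog tweaks are unconnected.
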(event Custom|SwapColors
  (bind _index (Variables|Default|Getindex))
  (bind _foginscatteringcolor (Variables|Default|GetFogInscatteringColor))
  (bind _postprocessingcolor (Variables|Default|GetPostProcessingColor))
  (Development|PrintString (Utilities|String|ToString(Integer) _index))
  (bind _postprocessingchange (Timeline|PostProceccingTimeline PlayFromStart)
    (:Update
      (bind _structout (Utilities|Struct|SetmembersinPostProcessSettings (Variables|/Script/Engine.CameraComponent|GetPostProcessSettings (Variables|Default|GetFollowCamera)) (Math|Color|Lerp(LinearColor) (Utilities|Array|Get(acopy) _postprocessingcolor _index) (Utilities|Array|Get(acopy) _postprocessingcolor (+ (Variables|Default|Getindex) 1)) _postprocessingchange)))
      (Timeline|FogTimeLine PlayFromStart
        (:Update
          (Class|ExponentialHeightFogComponent|SetDirectionalInscatteringColor (Variables|/Script/Engine.ExponentialHeightFog|GetComponent (Variables|Default|GetFog)) (Math|Color|Lerp(LinearColor) (Utilities|Array|Get(acopy) _foginscatteringcolor (Variables|Default|Getindex)) (Utilities|Array|Get(acopy) _foginscatteringcolor (+ (Variables|Default|Getindex) 1)) _postprocessingchange))
          (Variables|Default|SetStartLerping false))))))

(event Custom|OceanChange
  (if (not (Variables|Default|GetStartLerping))
    (if (< (Variables|Default|Getindex) (Utilities|Array|Length (Variables|Default|GetPostProcessingColor)))
      (Variables|Default|SetStartLerping true)
      (if (Variables|Default|GetStartLerping)
        (CallFunction|SwapColors)
        (if (not (Variables|Default|GetStartLerping))
          (Math|Integer|IncrementInt (Variables|Default|Getindex)
            (:%20%20
              (if (== (Variables|Default|Getindex) (Utilities|Array|Length (Variables|Default|GetPostProcessingColor)))
                (Variables|Default|Setindex 0)))))))))

(event EventBeginPlay
  (bind _asmy_gamemode (Utilities|Casting|CastToMyGamemode (Game|GetGameMode)))
  (bind _output_get (Variables|Default|SetGamemode _asmy_gamemode))
  (EventDispatchers|BindEventtoClimateChange _output_get (delegate Custom|OceanChange))
  (bind _output_get_2 (Variables|Default|SetPlayer (Game|Player|GetPlayerPawn 0)))
  (Development|PrintString (Utilities|GetDisplayName (Actor|GetComponentbyClass _output_get_2 "/Script/Engine.CameraComponent")))
  (bind _output_get_3 (Variables|Default|SetFollowCamera (Actor|GetComponentbyClass _output_get_2 "/Script/Engine.CameraComponent")))
  (Utilities|Struct|SetmembersinPostProcessSettings (Variables|/Script/Engine.CameraComponent|GetPostProcessSettings _output_get_3) "BM_SOG" "DOFM_Gaussian" 5e+03 (Utilities|Array|Get(acopy) (Variables|Default|GetPostProcessingColor)) 0.838095 -1.0 0.2 0 1.0 0.2 2.0 0.75 2e+02 7e+02 7e+03 2.5e+03)
  (bind _outactors (Actor|GetAllActorsOfClass "/Script/Engine.ExponentialHeightFog"))
  (if (> (Utilities|Array|Length _outactors) 0)
    (Variables|Default|SetFog (Utilities|Array|Get(acopy) _outactors))
    (Class|ExponentialHeightFogComponent|SetDirectionalInscatteringColor (Variables|/Script/Engine.ExponentialHeightFog|GetComponent (Variables|Default|GetFog)) (Utilities|Array|Get(acopy) (Variables|Default|GetFogInscatteringColor)))))

(event EventTick
  (params (DeltaSeconds :type Float%20%28single-precision%29)))

(event Collision|EventActorBeginOverlap
  (params (OtherActor :type Actor%20Object%20Reference)))

(fn ConstructionScript)