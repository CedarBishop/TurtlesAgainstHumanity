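; BP_ClimateChange is an actor meant to shift the scene's color tint on a camera as the climate changes.
; SwapColors plays a timeline that lerps the post-process SceneColorTint between adjacent Colors entries at Index, printing Index each update.
; The logic to cycle Index, get the turtle pawn's camera and bind to MyGamemode's climate event is disconnected, so nothing here triggers the swap.
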(event Custom|SwapColors
  (bind _colors (Variables|Default|GetColors))
  (bind _camera (Variables|Default|GetCamera))
  (bind _index (Variables|Default|GetIndex))
  (Utilities|IsValid _camera
    (:Is%20Valid
      (bind _colorchangetrack (Timeline|Timeline_0 PlayFromStart)
        (:Update
          (Utilities|Struct|SetmembersinPostProcessSettings (Variables|/Script/Engine.CameraComponent|GetPostProcessSettings _camera) (Math|Color|Lerp(LinearColor) (Utilities|Array|Get(acopy) _colors _index) (Utilities|Array|Get(acopy) _colors (+ (Variables|Default|GetIndex) 1)) _colorchangetrack))
          (Development|PrintString (Utilities|String|ToString(Integer) _index))
          (Variables|Default|SetStartLerping false))))))

(event EventBeginPlay)

(event Collision|EventActorBeginOverlap
  (params (OtherActor :type Actor%20Object%20Reference)))

(event EventTick
  (params (DeltaSeconds :type Float%20%28single-precision%29)))

(fn ConstructionScript)