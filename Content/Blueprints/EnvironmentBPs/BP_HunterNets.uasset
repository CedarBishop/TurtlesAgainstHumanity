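; BP_HunterNets is a net actor that traps a Player_Base actor on overlap.
; Beginning an overlap sets the player's IsStuckInNet flag, waits TimeStuckInNet, then clears the flag and destroys the net.
; Ending an overlap clears the flag immediately and resets TickCounter and IsOverlappingPlayer, while Tick only calls its parent.
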(event EventBeginPlay
  (|CallParentFunction) ; This node is disabled and will not be called.\nDrag off pins to build functionality.
)

(event Collision|EventActorBeginOverlap
  (params (OtherActor :type Actor%20Object%20Reference))
  (|CallParentFunction OtherActor)
  (bind _asplayer_base (Utilities|Casting|CastToPlayer_Base OtherActor))
  (bind _output_get (Variables|Default|SetPlayer_Base _asplayer_base))
  (Variables|/Script/VrTest.Player_Base|SetbIsStuckInNet _output_get true)
  (Utilities|FlowControl|Delay (Variables|Default|GetTimeStuckInNet))
  (Variables|/Script/VrTest.Player_Base|SetbIsStuckInNet (Variables|Default|GetPlayer_Base) false)
  (Actor|DestroyActor))

(event EventTick
  (params (DeltaSeconds :type Float%20%28single-precision%29))
  (|CallParentFunction DeltaSeconds))

(event Collision|EventActorEndOverlap
  (params (OtherActor :type Actor%20Object%20Reference))
  (bind _asplayer_base (Utilities|Casting|CastToPlayer_Base OtherActor))
  (Variables|/Script/VrTest.Player_Base|SetbIsStuckInNet _asplayer_base false)
  (Variables|Default|SetTickCounter 0)
  (Variables|Default|SetIsOverlappingPlayer false))

(fn ConstructionScript
  (|CallParentFunction))