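; PC-controlled player turtle that swims with left and right flipper inputs while managing stress and oxygen.
; Flipper, brake, obstacle-hit, resupply and stress events forward to functions defined outside this file, with camera axes driving controller rotation.
; Tick reports death to MyGamemode and runs delayed stress recovery.
; Also toggles pause through MyHud and refreshes SFX volume from the game instance when the gamemode signals settings changes.
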(event Custom|UnPause
  (bind _returnvalue (Game|GetPlayerController 0))
  (Game|SetGamePaused false)
  (Default|SetPauseState (Variables|Default|GetGameHud) false)
  (Input|SetInputModeGameOnly _returnvalue)
  (Variables|/Script/Engine.PlayerController|SetbShowMouseCursor _returnvalue false))

(event Custom|RaiseMinStress
  (params (AddedStress :type Float%20%28single-precision%29))
  (Class|PlayerBase|RaiseMinimumStressLevel AddedStress))

(event Custom|UpdateSFX
  (Class|PlayerBase|SetAudioComponentVolumes (Variables|/Game/Blueprints/CoreBPs/BP_GameInstance.BP_GameInstance_C|GetSfxVolume (Variables|Default|GetGameInstance))))

(event EventOnOxygenReSupply
  (params (StressHealed :type Float%20%28single-precision%29) (OxygenReplenished :type Float%20%28single-precision%29))
  (Class|PlayerBase|OxygenResupply StressHealed OxygenReplenished))

(event EventOnObstacleHit
  (params (StressDamage :type Float%20%28single-precision%29) (OxygenDamage :type Float%20%28single-precision%29))
  (Class|PlayerBase|ObstacleHit StressDamage OxygenDamage))

(event EventBeginPlay
  (bind _asmy_hud (Utilities|Casting|CastToMyHud (HUD|GetHUD (Game|GetPlayerController 0))))
  (Variables|Default|SetGameHud _asmy_hud)
  (bind _asmy_gamemode (Utilities|Casting|CastToMyGamemode (Game|GetGameMode)))
  (Variables|Default|SetGamemode _asmy_gamemode)
  (EventDispatchers|BindEventtoUpdateSettings _asmy_gamemode (delegate Custom|UpdateSFX))
  (bind _asbp_game_instance (Utilities|Casting|CastToBP_GameInstance (Game|GetGameInstance)))
  (bind _output_get (Variables|Default|SetGameInstance _asbp_game_instance))
  (Class|PlayerBase|SetAudioComponentVolumes (Variables|/Game/Blueprints/CoreBPs/BP_GameInstance.BP_GameInstance_C|GetSfxVolume _output_get)))

(event EventTick
  (params (DeltaSeconds :type Float%20%28single-precision%29))
  (Utilities|FlowControl|Sequence
    (:then_0
      (if (Variables|Default|GetbPlayerIsDead)
        (Default|PlayerDied (Variables|Default|GetGamemode))))
    (:then_1
      (Utilities|FlowControl|Delay 1.0)
      (Class|PlayerBase|StressRecovery))))

(event Input|ActionEvents|InputActionLeftFlipper
  (params (Key :type Key%20Structure))
  (:Pressed
    (Variables|ControllerBooleans|SetLeftFlipperDown true)
    (Class|PlayerBase|StartPcLeftCounter))
  (:Released
    (Variables|ControllerBooleans|SetLeftFlipperDown false)
    (Class|PlayerBase|EndPcLeftCounter)))

(event Input|ActionEvents|InputActionRightFlipper
  (params (Key :type Key%20Structure))
  (:Pressed
    (Variables|ControllerBooleans|SetRightFlipperDown true)
    (Class|PlayerBase|StartPcRightCounter))
  (:Released
    (Variables|ControllerBooleans|SetRightFlipperDown false)
    (Class|PlayerBase|EndPcRightCounter)))

(event Input|ActionEvents|InputActionBrake
  (params (Key :type Key%20Structure))
  (:Pressed
    (Class|PlayerBase|Brake))
  (:Released
    (Class|PlayerBase|UnBrake)))

(event Input|ActionEvents|InputActionPause
  (params (Key :type Key%20Structure))
  (bind _returnvalue (Game|GetPlayerController 0))
  (:Pressed
    (Game|SetGamePaused true)
    (Default|SetPauseState (Variables|Default|GetGameHud) true)
    (Input|SetInputModeUIOnly _returnvalue 0 "DoNotLock")
    (Variables|/Script/Engine.PlayerController|SetbShowMouseCursor _returnvalue true)))

(event Input|AxisEvents|InputAxisCameraX
  (params (AxisValue :type Float%20%28single-precision%29))
  (Pawn|Input|AddControllerYawInput (* AxisValue (Variables|Default|GetCameraX))))

(event Input|AxisEvents|InputAxisCameraY
  (params (AxisValue :type Float%20%28single-precision%29))
  (Pawn|Input|AddControllerPitchInput (* AxisValue (Variables|Default|GetCameraY))))

(fn ConstructionScript)